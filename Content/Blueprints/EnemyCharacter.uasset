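; Enemy character that repeatedly damages the hero while overlapping it and destroys itself when dead.
; Overlapping a HeroCharacter stores it and starts a looping timer, paced by AttacksPerSecond, that applies Damage through the hero's AffectHealth until overlap ends.
; Its own AffectHealth event runs CalculateHealth, prints Health and checks IsDead.
; The construction script tints the mesh with EnemyColor through a dynamic material instance.
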(event Custom|DamageTheHero
  (Default|AffectHealth (Variables|Default|GetHero) (Variables|Default|GetDamage)))

(event EventBeginPlay)

(event EventActorBeginOverlap
  (params (OtherActor :type Actor%20Object%20Reference))
  (bind _ashero_character (Utilities|Casting|CastToHeroCharacter OtherActor))
  (Variables|Default|SetHero _ashero_character)
  (bind _returnvalue (Utilities|Time|SetTimerbyFunctionName 0 "DamageTheHero" (/ 1.0 (Variables|Default|GetAttacksPerSecond)) true)))

(event EventTick
  (params (DeltaSeconds :type Float%20%28single-precision%29)))

(event EventAffectHealth
  (params (delta :type Float%20%28single-precision%29))
  (Class|BaseCharacter|CalculateHealth delta)
  (Development|PrintString (Utilities|String|ToString(Float) (Variables|Default|GetHealth)))
  (if (Variables|Default|GetisDead)
    (Actor|DestroyActor)))

(event Collision|EventActorEndOverlap
  (params (OtherActor :type Actor%20Object%20Reference))
  (if (== OtherActor (Variables|Default|GetHero))
    (Class|KismetSystemLibrary|ClearTimerHandle (stale EventActorBeginOverlap _returnvalue))))

(fn ConstructionScript
  (bind _returnvalue (Rendering|Material|CreateDynamicMaterialInstance (Variables|Character|GetMesh) 0 0 :!class /Script/Engine.PrimitiveComponent))
  (bind _output_get (Variables|Default|SetDynaMat _returnvalue))
  (Rendering|Material|SetVectorParameterValue _output_get "BodyColor" (Variables|Default|GetEnemyColor) :!class /Script/Engine.MaterialInstanceDynamic))