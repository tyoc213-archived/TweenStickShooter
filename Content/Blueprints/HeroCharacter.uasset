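; Player hero character with top-down, twin-stick-style controls that spawns a Weapon and attaches it to GunTemp on BeginPlay.
; Move axes drive movement along world X and Y.
; Both look axes share logic that, past a dead zone, sets control rotation and pulls the weapon trigger, otherwise releasing it.
; AffectHealth recalculates and prints health, destroying weapon and hero on death.
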(event EventBeginPlay
  (bind _guntemp (Variables|Default|GetGunTemp))
  (Utilities|FlowControl|Sequence
    (:then_0
      (bind _returnvalue (Game|SpawnActorfromClass "/Game/Blueprints/Weapon.Weapon_C" (Transformation|GetWorldTransform _guntemp) "Undefined" 0 0))
      (bind _output_get (Variables|Default|SetWeaponnnn _returnvalue))
      (Class|Actor|AttachRootComponentto _output_get _guntemp "None" "SnapToTarget" true))))

(event EventActorBeginOverlap
  (params (OtherActor :type Actor%20Object%20Reference)))

(event EventTick
  (params (DeltaSeconds :type Float%20%28single-precision%29)))

(event EventAffectHealth
  (params (delta :type Float%20%28single-precision%29))
  (Class|BaseCharacter|CalculateHealth delta)
  (Development|PrintString (Utilities|String|ToString(Float) (Variables|Default|GetHealth)))
  (if (Variables|Default|GetisDead)
    (Actor|DestroyActor (Variables|Default|GetWeaponnnn))))

(event Input|AxisEvents|InputAxisLookUp
  (params (AxisValue :type Float%20%28single-precision%29))
  (bind _weaponnnn (Variables|Default|GetWeaponnnn))
  (if (> (Math|Vector|VectorLength (Math|Vector|MakeVector AxisValue (stale Input|AxisEvents|InputAxisLookRight AxisValue) 0.0)) 0.25)
    (Pawn|SetControlRotation (Pawn|GetController) (Math|Conversions|RotationFromXVector (Math|Vector|MakeVector AxisValue (stale Input|AxisEvents|InputAxisLookRight AxisValue) 0.0)))
    (Default|PullTrigger _weaponnnn)
    (else
      (Default|ReleaseTrigger _weaponnnn))))

(event Input|AxisEvents|InputAxisLookRight
  (params (AxisValue :type Float%20%28single-precision%29))
  (bind _weaponnnn (Variables|Default|GetWeaponnnn))
  (if (> (Math|Vector|VectorLength (Math|Vector|MakeVector (stale Input|AxisEvents|InputAxisLookUp AxisValue) AxisValue 0.0)) 0.25)
    (Pawn|SetControlRotation (Pawn|GetController) (Math|Conversions|RotationFromXVector (Math|Vector|MakeVector (stale Input|AxisEvents|InputAxisLookUp AxisValue) AxisValue 0.0)))
    (Default|PullTrigger _weaponnnn)
    (else
      (Default|ReleaseTrigger _weaponnnn))))

(event Input|AxisEvents|InputAxisMoveUp
  (params (AxisValue :type Float%20%28single-precision%29))
  ;[1 1 1] Axis movement
  (Pawn|Input|AddMovementInput "1.000000,0.000000,0.000000" AxisValue false))

(event Input|AxisEvents|InputAxisMoveRight
  (params (AxisValue :type Float%20%28single-precision%29))
  ;[1 1 1] Axis movement
  (Pawn|Input|AddMovementInput "0.000000,1.000000, 0" AxisValue false))

(fn ConstructionScript)